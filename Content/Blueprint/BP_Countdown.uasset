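; BP_Countdown is a countdown timer actor that starts from TimeInSeconds when play begins.
; Each Tick subtracts DeltaSeconds from CurrentTimeInSeconds, clamps it at zero and prints the formatted time to screen for one frame.
; It then fires the OnTimeUpdate dispatcher every frame, including after the count reaches zero, with no separate completion event.
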(event `self.ReceiveBeginPlay`
  (set `self.CurrentTimeInSeconds` (`self.TimeInSeconds`)))

(event `self.ReceiveTick`
  (params (DeltaSeconds :type "Float (single-precision)"))
  (bind _output_get (set `self.CurrentTimeInSeconds` (`KismetMathLibrary.FClamp` (- (`self.CurrentTimeInSeconds`) DeltaSeconds) 0.0 (`self.CurrentTimeInSeconds`))))
  (`KismetSystemLibrary.PrintString` (`KismetStringLibrary.TimeSecondsToString` _output_get) true false (struct :`G` 0.66 :`B` 1.0 :`A` 1.0) DeltaSeconds)
  (`self.OnTimeUpdate`))

(fn `UserConstructionScript`)
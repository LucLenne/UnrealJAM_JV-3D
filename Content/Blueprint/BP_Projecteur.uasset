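; BP_Projecteur is a projector actor that casts an image through three spot lights, R, G and B, using anamorphosis light function materials.
; The construction script creates a dynamic instance of the red, green or blue material for each light and passes it the Image texture, since each light handles one color channel.
; It also applies a shared intensity and outer cone angle to all three lights; the event graph is empty.
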(fn `UserConstructionScript`
  (bind _returnvalue (`KismetMaterialLibrary.CreateDynamicMaterialInstance` "/Game/Asset/Material/M_AnamorphoseBlue.M_AnamorphoseBlue"))
  (`MaterialInstanceDynamic.SetTextureParameterValue` _returnvalue "Image" (`self.Image`))
  (`LightComponent.SetLightFunctionMaterial` (`self.B`) _returnvalue)
  (bind _returnvalue_2 (`KismetMaterialLibrary.CreateDynamicMaterialInstance` "/Game/Asset/Material/M_AnamorphoseGreen.M_AnamorphoseGreen"))
  (`MaterialInstanceDynamic.SetTextureParameterValue` _returnvalue_2 "Image" (`self.Image`))
  (`LightComponent.SetLightFunctionMaterial` (`self.G`) _returnvalue_2)
  (bind _returnvalue_3 (`KismetMaterialLibrary.CreateDynamicMaterialInstance` "/Game/Asset/Material/M_AnamorphoseRed.M_AnamorphoseRed"))
  (`MaterialInstanceDynamic.SetTextureParameterValue` _returnvalue_3 "Image" (`self.Image`))
  (`LightComponent.SetLightFunctionMaterial` (`self.R`) _returnvalue_3)
  (`LightComponent.SetIntensity` (`self.R`) (`self.IntensityLight`))
  (`LightComponent.SetIntensity` (`self.G`) (`self.IntensityLight`))
  (`LightComponent.SetIntensity` (`self.B`) (`self.IntensityLight`))
  (`SpotLightComponent.SetOuterConeAngle` (`self.R`) (`self.OuterConeAngle`))
  (`SpotLightComponent.SetOuterConeAngle` (`self.G`) (`self.OuterConeAngle`))
  (`SpotLightComponent.SetOuterConeAngle` (`self.B`) (`self.OuterConeAngle`)))
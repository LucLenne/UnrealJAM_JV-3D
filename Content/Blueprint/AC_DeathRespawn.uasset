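; AC_DeathRespawn is an actor component that handles death and checkpoint respawn for its owner.
; On BeginPlay it stores the owner's location as the last checkpoint if that variable is still near zero.
; CE_Die prints a debug message and calls respawn after a short delay, which teleports the owner to the stored location without sweeping.
; Nothing in this graph updates the checkpoint after BeginPlay.
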(event `self.ReceiveBeginPlay`
  (if (== (`self.LastCheckPointLocation`) (`KismetMathLibrary.Vector_Zero`) :`ErrorTolerance` 1.0)
    (set `self.LastCheckPointLocation` (`Actor.K2_GetActorLocation` (`self.GetOwner`)))))

(event `CE_Die`
  (`KismetSystemLibrary.PrintString` "Là c'est Die")
  (`KismetSystemLibrary.Delay` 3.0)
  (`self.CE_Respaw`))

(event `CE_Respaw`
  (`Actor.K2_SetActorLocation` (`self.GetOwner`) (`self.LastCheckPointLocation`) false true))
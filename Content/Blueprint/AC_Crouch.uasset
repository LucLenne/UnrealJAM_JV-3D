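; Actor component that toggles crouching for the first-person player character.
; On BeginPlay it casts its owner to BP_FirstPersonCharacter and caches it, printing an error if the cast fails.
; CE_Crouch flips the character between Crouch and UnCrouch, tracks an IsCrouching flag and plays an optional 2D sound on each toggle.
; CE_ResetCrouch forces standing and clears the flag without sound.
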(event `self.ReceiveBeginPlay`
  (`self.BP_Player`
    (:`then`)
    (:`else`
      (bind _asbp_first_person_character (cast `/Game/FirstPerson/Blueprints/BP_FirstPersonCharacter` (`self.GetOwner`))
        (:`then`
          (set `self.BP_Player` _asbp_first_person_character))
        (:`CastFailed`
          (`KismetSystemLibrary.PrintString` "Owner is not a FirstPersonCharacter"))))))

(event `CE_Crouch`
  (bind _bp_player (`self.BP_Player`))
  (if (`self.IsCrouching`)
    (`Character.UnCrouch` _bp_player)
    (set `self.IsCrouching` false)
    (else
      (`Character.Crouch` _bp_player)
      (set `self.IsCrouching` true)))
  (bind _crouchsound (`self.CrouchSound`)
    (:`then`
      (`GameplayStatics.PlaySound2D` _crouchsound 1.0 1.0 0.0 null null))
    (:`else`)))

(event `CE_ResetCrouch`
  (`Character.UnCrouch` (`self.BP_Player`))
  (set `self.IsCrouching` false))
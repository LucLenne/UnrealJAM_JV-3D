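; BP_StairsManager is an actor that builds a vertical stack of BPStair actors when play begins.
; BeginPlay triggers a custom spawn event that loops from zero through Level, spawning one stair per index.
; Each stair copies the manager's transform, raised in Z by the index times StairHeight, and always spawns regardless of collision.
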(event `self.ReceiveBeginPlay`
  (`self.CE_Spawn`))

(event `CE_Spawn`
  (bind _returnvalue (`self.GetTransform`))
  (for _index (range (+ (`self.Level`) 1))
    (`|SpawnActorFromClass` (`self.BP_Stair`) (`KismetMathLibrary.MakeTransform` (`KismetMathLibrary.MakeVector` (.x (.location _returnvalue)) (.y (.location _returnvalue)) (+ (.z (.location _returnvalue)) (* _index (`self.StairHeight`)))) (.rotation _returnvalue) (.scale _returnvalue)) "AlwaysSpawn" "MultiplyWithRoot" null null)))

(fn `UserConstructionScript`)
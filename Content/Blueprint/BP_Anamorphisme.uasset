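; Anamorphosis puzzle actor that reveals a key object when the player finds the right viewpoint and viewing direction.
; The construction script projects one image through four spotlights (R, G, B, A) using dynamic light-function materials, scales the view-angle target and hides the key.
; While the player overlaps GoodPosition, Tick line-traces from the first-person camera.
; A hit locks input, blends to a puzzle camera, reveals the key, restores control and destroys the actor.
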(event `self.ReceiveBeginPlay`
  (bind _asbp_first_person_character (cast `/Game/FirstPerson/Blueprints/BP_FirstPersonCharacter` (`GameplayStatics.GetPlayerCharacter` 0)))
  (set `self.First Person Camera` (`/Game/FirstPerson/Blueprints/BP_FirstPersonCharacter.FirstPersonCamera` _asbp_first_person_character)))

(event `self.GoodPosition.OnComponentBeginOverlap`
  (params (OverlappedComponent :type "PrimitiveComponent Object Reference") (OtherActor :type "Actor Object Reference") (OtherComp :type "PrimitiveComponent Object Reference") (OtherBodyIndex :type Integer) (bFromSweep :type Boolean) (SweepResult :type "HitResult Structure (by ref)"))
  ;[0.1594 0.1594 0.1594] Overlap
  (set `self.Overlap` true))

(event `self.GoodPosition.OnComponentEndOverlap`
  (params (OverlappedComponent :type "PrimitiveComponent Object Reference") (OtherActor :type "Actor Object Reference") (OtherComp :type "PrimitiveComponent Object Reference") (OtherBodyIndex :type Integer))
  ;[0.1594 0.1594 0.1594] Overlap
  (set `self.Overlap` false))

(event `self.ReceiveTick`
  (params (DeltaSeconds :type "Float (single-precision)"))
  (bind _returnvalue (`GameplayStatics.GetPlayerController` 0))
  (bind _returnvalue_2 (`GameplayStatics.GetPlayerController` 0))
  (bind _first_person_camera (`self.First Person Camera`))
  (bind _bp_objectkey (`self.BP_ObjectKey`))
  (bind _bp_objectkey_2 (`self.BP_ObjectKey`))
  (bind _returnvalue_3 (`SceneComponent.K2_GetComponentLocation` _first_person_camera))
  ;[0.1344 0.1344 0.1344] Trance line in front of player
  (if (`self.Overlap`)
    (bind (_outhit _returnvalue_4) (`KismetSystemLibrary.LineTraceSingle` :`Start` _returnvalue_3 :`End` (+ (* (`SceneComponent.GetForwardVector` _first_person_camera) 2500.0) _returnvalue_3) :`TraceChannel` "TraceTypeQuery3" :`DrawDebugType` "ForDuration" :`bIgnoreSelf` false))
    (if _returnvalue_4
      (`/Engine/EditorBlueprintResources/StandardMacros.DoOnce` false
        (:`Completed`
          (`GameplayStatics.PlaySound2D` "/Game/Asset/SD/SFX_validation.SFX_validation" 1.0 1.0 0.0 null null)
          (`self.DisableInput` (`Controller.K2_GetPawn` _returnvalue) _returnvalue)
          ;[0.1135 0.1135 0.1135] Transition Camera
          (`PlayerController.SetViewTargetWithBlend` _returnvalue (`ActorComponent.GetOwner` (`self.CameraAnamorhisme`)) 2.0 "VTBlend_Linear" 0.0 true)
          (`KismetSystemLibrary.Delay` 3.0)
          (`GameplayStatics.PlaySound2D` "/Game/Asset/SD/SFX_object_spawn.SFX_object_spawn" 1.0 1.0 0.0 null null)
          ;[0.1135 0.1135 0.1135] Spawn key
          (`/Engine/EditorBlueprintResources/StandardMacros.IsValid` _bp_objectkey
            (:`Is Valid`
              (`self.SetActorHiddenInGame` _bp_objectkey false)
              ;[0.1719 0.1719 0.1719] Return on camera player
              (`PlayerController.SetViewTargetWithBlend` (`GameplayStatics.GetPlayerController` 0) (`GameplayStatics.GetPlayerCharacter` 0) 2.0 "VTBlend_Linear" 0.0 true)
              (`KismetSystemLibrary.Delay` 3.0)
              (`self.EnableInput` (`Controller.K2_GetPawn` _returnvalue_2) _returnvalue_2)
              (`PrimitiveComponent.SetCollisionEnabled` (`/Game/Blueprint/KeyObject/BP_ObjectKey.ObjectToChange` _bp_objectkey_2) "QueryAndPhysics")
              (`self.SetActorHiddenInGame` _bp_objectkey_2 false)
              (`self.K2_DestroyActor` self))
            (:`Is Not Valid`
              (`KismetSystemLibrary.PrintString` "object key missing" true true (struct :`G` 0.66 :`B` 1.0 :`A` 1.0) 5.0))))))))

(fn `UserConstructionScript`
  (bind _bp_objectkey (`self.BP_ObjectKey`))
  (bind _precisionforanamorphisme (`self.PrecisionForAnamorphisme`))
  ;[0.1552 0.1552 0.1552] Apply an image to all spotlight
  (bind _returnvalue (`KismetMaterialLibrary.CreateDynamicMaterialInstance` "/Game/Asset/Material/M_AnamorphoseBlue.M_AnamorphoseBlue"))
  (`MaterialInstanceDynamic.SetTextureParameterValue` _returnvalue "Image" (`self.Image`))
  (`LightComponent.SetLightFunctionMaterial` (`self.B`) _returnvalue)
  (bind _returnvalue_2 (`KismetMaterialLibrary.CreateDynamicMaterialInstance` "/Game/Asset/Material/M_AnamorphoseGreen.M_AnamorphoseGreen"))
  (`MaterialInstanceDynamic.SetTextureParameterValue` _returnvalue_2 "Image" (`self.Image`))
  (`LightComponent.SetLightFunctionMaterial` (`self.G`) _returnvalue_2)
  (bind _returnvalue_3 (`KismetMaterialLibrary.CreateDynamicMaterialInstance` "/Game/Asset/Material/M_AnamorphoseRed.M_AnamorphoseRed"))
  (`MaterialInstanceDynamic.SetTextureParameterValue` _returnvalue_3 "Image" (`self.Image`))
  (`LightComponent.SetLightFunctionMaterial` (`self.R`) _returnvalue_3)
  (bind _returnvalue_4 (`KismetMaterialLibrary.CreateDynamicMaterialInstance` "/Game/Asset/Material/M_AnamorphoseAlpha.M_AnamorphoseAlpha"))
  (`MaterialInstanceDynamic.SetTextureParameterValue` _returnvalue_4 "Image" (`self.Image`))
  (`LightComponent.SetLightFunctionMaterial` (`self.A`) _returnvalue_4)
  ;[0.1385 0.1385 0.1385] Set intensity & outer cone angle
  (`LightComponent.SetIntensity` (`self.R`) (`self.IntensityLight`))
  (`LightComponent.SetIntensity` (`self.G`) (`self.IntensityLight`))
  (`LightComponent.SetIntensity` (`self.B`) (`self.IntensityLight`))
  (`LightComponent.SetIntensity` (`self.A`) (`self.IntensityLight`))
  (`SpotLightComponent.SetOuterConeAngle` (`self.R`) (`self.OuterConeAngle`))
  (`SpotLightComponent.SetOuterConeAngle` (`self.G`) (`self.OuterConeAngle`))
  (`SpotLightComponent.SetOuterConeAngle` (`self.B`) (`self.OuterConeAngle`))
  (`SpotLightComponent.SetOuterConeAngle` (`self.A`) (`self.OuterConeAngle`))
  ;[0.1344 0.1344 0.1344] Set Key object
  (`PrimitiveComponent.SetCollisionEnabled` (`/Game/Blueprint/KeyObject/BP_ObjectKey.ObjectToChange` _bp_objectkey) "NoCollision")
  (`self.SetActorHiddenInGame` _bp_objectkey true)
  (`SceneComponent.SetWorldScale3D` (`self.GoodViewAngle`) (`KismetMathLibrary.MakeVector` _precisionforanamorphisme _precisionforanamorphisme _precisionforanamorphisme)))
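; BP_Door is a door that opens when a BP_ObjectKey comes within range.
; Every Tick it runs a box overlap at CheckKeyAround, destroys each key found, rotates the Door mesh 90 degrees and disables its collision.
; It then plays a 2D open sound, printing debug messages if the sound or mesh is missing.
; The construction script applies the configurable MeshDoor to the Door component.
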(event `self.ReceiveTick`
  (params (DeltaSeconds :type "Float (single-precision)"))
  (bind _sounddooropen (`self.SoundDoorOpen`))
  (bind _door (`self.Door`))
  (bind _outactors (`KismetSystemLibrary.BoxOverlapActors` (`SceneComponent.K2_GetComponentLocation` (`self.CheckKeyAround`)) (100.0 100.0 100.0) (`self.Object Types`) "/Game/Blueprint/KeyObject/BP_ObjectKey.BP_ObjectKey_C"))
  (for _array_element _outactors
    (bind _asbp_object_key (cast `/Game/Blueprint/KeyObject/BP_ObjectKey` _array_element))
    (`self.K2_DestroyActor` _asbp_object_key)
    (`/Engine/EditorBlueprintResources/StandardMacros.IsValid` _door
      (:`Is Valid`
        (`SceneComponent.K2_AddWorldRotation` _door (struct :`Yaw` 90.0) false false)
        (`PrimitiveComponent.SetCollisionEnabled` _door "NoCollision")
        (`/Engine/EditorBlueprintResources/StandardMacros.IsValid` _sounddooropen
          (:`Is Valid`
            (`GameplayStatics.PlaySound2D` _sounddooropen 1.0 1.0 0.0 null null))
          (:`Is Not Valid`
            (`KismetSystemLibrary.PrintString` "sound door not implemented" true true (struct :`G` 0.66 :`B` 1.0 :`A` 1.0) 5.0))))
      (:`Is Not Valid`
        (`KismetSystemLibrary.PrintString` "Mesh door missing" true true (struct :`G` 0.66 :`B` 1.0 :`A` 1.0) 5.0)))))

(fn `UserConstructionScript`
  (`StaticMeshComponent.SetStaticMesh` (`self.Door`) (`self.MeshDoor`)))
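; BP_CheckPoint is a checkpoint that saves game state for respawning when its overlap component is triggered.
; It caches the first-person character on first contact, then writes its own location to that character's AC_DeathRespawn component.
; It also stores BP_Monster's location and BP_Countdown's remaining time, using the temporary time value while the countdown is glitching.
; An optional flag destroys the checkpoint afterwards.
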(event `self.CheckPoint.OnComponentBeginOverlap`
  (params (OverlappedComponent :type "PrimitiveComponent Object Reference") (OtherActor :type "Actor Object Reference") (OtherComp :type "PrimitiveComponent Object Reference") (OtherBodyIndex :type Integer) (bFromSweep :type Boolean) (SweepResult :type "HitResult Structure (by ref)"))
  (`self.BP_Player`
    (:`then`
      (bind _returnvalue (`self.GetComponentByClass` (stale _output_get) "/Game/Blueprint/AC_DeathRespawn.AC_DeathRespawn_C"))
      (`/Engine/EditorBlueprintResources/StandardMacros.IsValid` _returnvalue :!label _label
        (:`Is Valid`
          (set `/Game/Blueprint/AC_DeathRespawn.LastCheckPointLocation` (`self.K2_GetActorLocation`) _returnvalue))
        (:`Is Not Valid`
          (`KismetSystemLibrary.PrintString` "No Death Respawn Component found")))
      (bind _returnvalue_2 (`GameplayStatics.GetActorOfClass` "/Game/Blueprint/AI/BP_Monster.BP_Monster_C"))
      (`/Engine/EditorBlueprintResources/StandardMacros.IsValid` _returnvalue_2
        (:`Is Valid`
          (set `/Game/Blueprint/AC_DeathRespawn.MonsterLocationOnChekpoint` (`self.K2_GetActorLocation` _returnvalue_2) _returnvalue))
        (:`Is Not Valid`
          (`KismetSystemLibrary.PrintString` "Monster not found")))
      (bind _returnvalue_3 (`GameplayStatics.GetActorOfClass` "/Game/Blueprint/BP_Countdown.BP_Countdown_C"))
      (`/Engine/EditorBlueprintResources/StandardMacros.IsValid` _returnvalue_3
        (:`Is Valid`
          (if (`/Game/Blueprint/BP_Countdown.IsGlitching` _returnvalue_3)
            (set `/Game/Blueprint/AC_DeathRespawn.TimeLeftOnCheckPoint` (`/Game/Blueprint/BP_Countdown.TempCurrentTimeInSeconds` _returnvalue_3) _returnvalue)
            (else
              (set `/Game/Blueprint/AC_DeathRespawn.TimeLeftOnCheckPoint` (`/Game/Blueprint/BP_Countdown.CurrentTimeInSeconds` _returnvalue_3) _returnvalue))))
        (:`Is Not Valid`
          (`KismetSystemLibrary.PrintString` "Countdown not found")))
      (if (`self.DestroyAfterCheking`)
        (`self.K2_DestroyActor`)))
    (:`else`
      (bind _asbp_first_person_character (cast `/Game/FirstPerson/Blueprints/BP_FirstPersonCharacter` OtherActor)
        (:`then`
          (bind _output_get (set `self.BP_Player` _asbp_first_person_character))
          (goto _label))
        (:`CastFailed`
          (`KismetSystemLibrary.PrintString` "Cast Checkpoint Player Failed"))))))

(fn `UserConstructionScript`)
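; AC_Flashlight is an actor component that dims and shortens its owner's flashlight as the level countdown runs down.
; On BeginPlay it uses the assigned light or finds the owner's SpotLightComponent, locates BP_Countdown, and sets intensity and attenuation radius to maximum.
; It binds to the countdown's time update, rescaling both values through macros that lerp from zero to maximum by remaining-time fraction.
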(event `self.ReceiveBeginPlay`
  (bind _flashlight (`self.FlashLight`))
  (bind _returnvalue (`Actor.GetComponentByClass` (`self.GetOwner`) "/Script/Engine.SpotLightComponent"))
  (`self.FlashLight`
    (:`then`
      (bind _returnvalue_2 (`GameplayStatics.GetActorOfClass` "/Game/Blueprint/BP_Countdown.BP_Countdown_C" :!label _label))
      (`/Engine/EditorBlueprintResources/StandardMacros.IsValid` _returnvalue_2
        (:`Is Valid`
          (bind _output_get (set `self.BP_CountDown` _returnvalue_2))
          (add `/Game/Blueprint/BP_Countdown.OnTimeUpdate` _output_get (delegate `UpdateFlashlight`))
          (`LightComponent.SetIntensity` _flashlight (`self.MaxIntensity`))
          (`LocalLightComponent.SetAttenuationRadius` _flashlight (`self.MaxAttenuationRadius`)))
        (:`Is Not Valid`
          (`KismetSystemLibrary.PrintString` "No count down place in world"))))
    (:`else`
      (`/Engine/EditorBlueprintResources/StandardMacros.IsValid` _returnvalue
        (:`Is Valid`
          (set `self.FlashLight` _returnvalue)
          (goto _label))
        (:`Is Not Valid`
          (`KismetSystemLibrary.PrintString` "No flashLight on character"))))))

(event `UpdateFlashlight`
  (bind _flashlight (`self.FlashLight`))
  (`LightComponent.SetIntensity` _flashlight (`self.M_LerpIntensity`))
  (`LocalLightComponent.SetAttenuationRadius` _flashlight (`self.M_LerpAttenuationRadius`)))
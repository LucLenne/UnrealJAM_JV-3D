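; BP_Monster is an AI monster that closes in on the player as the level countdown runs out and kills them if they linger too close.
; Each BP_Countdown update lerps the allowed follow distance by remaining time and writes it, minus the player's capsule radius, to the Blackboard.
; An attack sphere sized by AttackRange runs a timer on Tick that calls the player's death/respawn component, resetting when the player leaves.
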(event `self.ReceiveBeginPlay`
  (`self.Player`
    (:`then`
      _)
    (:`else`
      (bind _asbp_first_person_character (cast `/Game/FirstPerson/Blueprints/BP_FirstPersonCharacter` (`GameplayStatics.GetPlayerCharacter` 0)))
      (set `self.Player` _asbp_first_person_character)))
  (`self.M_UpdateMinDistance` (`self.DistanceFromPlayer`))
  (`KismetArrayLibrary.Array_Add` (`self.LocationHistory`) (`self.K2_GetActorLocation`))
  (bind _returnvalue (`GameplayStatics.GetActorOfClass` "/Game/Blueprint/BP_Countdown.BP_Countdown_C"))
  (bind _output_get (set `self.BP_Countdown` _returnvalue))
  (add `/Game/Blueprint/BP_Countdown.OnTimeUpdate` _output_get (delegate `UpdateMinDistance`))
  (`self.M_SetTimeBeforeAttacking`))

(event `UpdateMinDistance`
  (bind _bp_countdown (`self.BP_Countdown`))
  (`self.M_UpdateMinDistance` (`KismetMathLibrary.Lerp` (`self.MinDistanceFromPlayer`) (`self.DistanceFromPlayer`) (/ (`/Game/Blueprint/BP_Countdown.CurrentTimeInSeconds` _bp_countdown) (`/Game/Blueprint/BP_Countdown.TimeInSeconds` _bp_countdown)))))

(event `self.ReceiveTick`
  (params (DeltaSeconds :type "Float (single-precision)"))
  (if (`self.IsPlayerInAttackRange`)
    (bind _output_get (set `self.TempTimeBeforeAttacking` (- (`self.TempTimeBeforeAttacking`) DeltaSeconds)))
    (if (<= _output_get 0.0)
      (`self.CE_AttackPlayer`))
    (elif (!= (`self.TimeBeforeAttacking`) (`self.TempTimeBeforeAttacking`))
      (`self.M_SetTimeBeforeAttacking`))))

(event `CE_AttackPlayer`
  (`/Game/Blueprint/AC_DeathRespawn.CE_Die` (`/Game/FirstPerson/Blueprints/BP_FirstPersonCharacter.AC_DeathRespawn` (`self.Player`))))

(event `self.AttackZone.OnComponentBeginOverlap`
  (params (OverlappedComponent :type "PrimitiveComponent Object Reference") (OtherActor :type "Actor Object Reference") (OtherComp :type "PrimitiveComponent Object Reference") (OtherBodyIndex :type Integer) (bFromSweep :type Boolean) (SweepResult :type "HitResult Structure (by ref)"))
  (if (== OtherActor (`self.Player`))
    (set `self.IsPlayerInAttackRange` true)))

(event `self.AttackZone.OnComponentEndOverlap`
  (params (OverlappedComponent :type "PrimitiveComponent Object Reference") (OtherActor :type "Actor Object Reference") (OtherComp :type "PrimitiveComponent Object Reference") (OtherBodyIndex :type Integer))
  (if (== OtherActor (`self.Player`))
    (set `self.IsPlayerInAttackRange` false)))

(fn `UserConstructionScript`
  (`SphereComponent.SetSphereRadius` (`self.AttackZone`) (`self.AttackRange`) true))